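; BP_Jill is an AI-controlled character whose chase state follows the player's inventory.
; On BeginPlay it enables chasing, then binds an event to the CanBeChased dispatcher on the player ThirdPersonCharacter's CharInventory.
; The Chasing function stores the flag and writes it to the bChase blackboard key through its NPC_AI controller.
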(event `self.ReceiveBeginPlay`
  (`self.Chasing` true)
  (bind _asthird_person_character (cast `/Game/Blueprint/ThirdPersonCharacter` (`GameplayStatics.GetPlayerCharacter` 0)))
  (add `InventoryComponent.CanBeChased` (`HeroCraftCharacter.CharInventory` _asthird_person_character) (`|CreateDelegate` :!event `Chasing`)))

(fn `Chasing`
  (params (bCanBeChased :type Boolean))
  (bind _output_get (set `self.bIsChasing` bCanBeChased))
  (bind _asnpc_ai (cast `/Game/AI/NPC_AI` (`self.GetController`)))
  (`BlackboardComponent.SetValueAsBool` (`AIBlueprintHelperLibrary.GetBlackboard` _asnpc_ai) "bChase" _output_get))

(fn `UserConstructionScript`)